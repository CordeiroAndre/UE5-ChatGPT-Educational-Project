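; BP_ComputerGameplay is the in-game computer actor that shows the selected character's portrait on its screen.
; On BeginPlay it puts a dynamic material on the screen plane, fed by the portrait from CharacterDataHolderSubsystem.
; When the pop-up sequence finishes, it tells HUD_Gameplay to create its widgets.
; From then on, Tick bobs and rolls the mesh with sine waves around its initial height.
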(event Custom|OnFinished_Event_0
  (Variables|Default|SetFinishedIntroAnimation true)
  (bind _ashud_gameplay (Utilities|Casting|CastToHUD_Gameplay (HUD|GetHUD (Game|GetPlayerController 0))))
  (Default|CreateWidgets _ashud_gameplay))

(event EventBeginPlay
  (Utilities|FlowControl|Sequence
    (:then_0
      (bind _returnvalue (Rendering|Material|CreateDynamicMaterialInstance (Variables|Default|GetPlane) 0 "/Game/HistoricalFigures/Computer/M_ComputerScreenGameplay.M_ComputerScreenGameplay" "None" :!class /Script/Engine.PrimitiveComponent))
      (Rendering|Material|SetTextureParameterValue _returnvalue "Texture" (.portrait (Variables|/Script/HistoricalFigures.CharacterDataHolderSubsystem|GetSelectedCharacterDescription (Subsystems|GetCharacterDataHolderSubsystem))))
      (Rendering|Material|SetScalarParameterValue _returnvalue "NumberOfColumns" (Math|Conversions|ToFloat(Integer) 0) :!class /Script/Engine.MaterialInstanceDynamic)
      (Rendering|Material|SetMaterial (Variables|Default|GetPlane) 0 _returnvalue))
    (:then_1
      (EventDispatchers|AssignOnFinished (Variables|/Script/ActorSequence.ActorSequenceComponent|GetSequencePlayer (Variables|Default|GetPopUpSequence)) (delegate Custom|OnFinished_Event_0))
      (Variables|Default|SetInitialLocation (.z (Variables|/Script/Engine.SceneComponent|GetRelativeLocation (Variables|Default|GetStaticMesh)))))))

(event EventTick
  (params (DeltaSeconds :type Float%20%28single-precision%29))
  (if (Variables|Default|GetFinishedIntroAnimation)
    (Transformation|SetRelativeLocation (Variables|Default|GetStaticMesh) (Math|Vector|MakeVector 0.0 0.0 (+ (Variables|Default|GetInitialLocation) (* (Math|Trig|Sin(Radians) (* (Utilities|Time|GetGameTimeinSeconds) 5.0)) 3.0))) false false)
    (Transformation|SetRelativeRotation (Variables|Default|GetStaticMesh) (Math|Rotator|MakeRotator (* (Math|Trig|Sin(Radians) (* (Utilities|Time|GetGameTimeinSeconds) 3.0)) -1.5) 0.0 0.0) false false)))

(fn ConstructionScript)