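; PC_Gameplay is the gameplay player controller for the HistoricalFigures game, handling the pause menu and message submission.
; Escape calls PauseGame, where a FlipFlop toggles both the game's paused state and the menu visibility on HUD_Gameplay.
; SendMessage stores the supplied text as the current recognized text and confirms speech recognition, so messages enter the same path as recognized speech.
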(event Custom|PauseGame
  (bind _isa (Utilities|FlowControl|FlipFlop)
    (:A
      _)
    (:B
      _))
  (Game|SetGamePaused _isa)
  (Default|SetMenuVisible (.AsHUD%20Gameplay (Utilities|Casting|CastToHUD_Gameplay (HUD|GetHUD))) _isa))

(event Custom|Send%20Message
  (params (Message :type String))
  (Variables|Default|SetCurrentRecognizedText Message)
  (Class|HFPlayerController|ConfirmSpeechRecognition (Class|KismetSystemLibrary|MakeLiteralBool true)))

(event Input|KeyboardEvents|Escape
  (params (Key :type Key%20Structure :default "None"))
  (:Pressed
    (CallFunction|PauseGame)))

(fn ConstructionScript)