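; BP_BookOpened is an actor, named as an opened book for the library sequences, that bobs gently up and down in place.
; BeginPlay stores the root component's world location as a base position.
; Each Tick sets the root to that base plus a small vertical sine offset driven by game time, without sweeping.
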(event EventBeginPlay
  (Variables|Default|SetRelative%20Location (Transformation|GetWorldLocation (Variables|Default|GetDefaultSceneRoot))))

(event EventTick
  (params (DeltaSeconds :type Float%20%28single-precision%29))
  (Transformation|SetWorldLocation (Variables|Default|GetDefaultSceneRoot) (+ (Variables|Default|GetRelative%20Location) (Math|Vector|MakeVector 0.0 0.0 (* (Math|Trig|Sin(Radians) (Utilities|Time|GetGameTimeinSeconds)) 3.0))) false false))

(fn ConstructionScript)